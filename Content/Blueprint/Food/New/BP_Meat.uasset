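; BP_Meat is a food actor that cooks while its mesh overlaps an actor whose display name is exactly "BP_Grill".
; If CanCook is set and it is not overcooked, overlap creates a dynamic Meat material and plays a timeline driving its Color and CookRate.
; Leaving the grill stops the timeline, so re-entry resumes from that point, and reaching the end sets IsOvercooked.
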(event `self.Static Mesh.OnComponentBeginOverlap`
  (params (OverlappedComponent :type "PrimitiveComponent Object Reference") (OtherActor :type "Actor Object Reference") (OtherComp :type "PrimitiveComponent Object Reference") (OtherBodyIndex :type Integer) (bFromSweep :type Boolean) (SweepResult :type "HitResult Structure (by ref)"))
  (if (`self.canCook`)
    (if (`KismetStringLibrary.EqualEqual_StrStr` "BP_Grill" (`KismetSystemLibrary.GetDisplayName` OtherActor))
      (if (not (`self.isOvercooked`))
        (bind _returnvalue (`PrimitiveComponent.CreateDynamicMaterialInstance` (`self.Static Mesh`) 0 "/Game/Assets/Food/meat.meat" "None"))
        (bind (_direction _cookcolor _cookfloat) (`Timeline|Timeline` :!label _label)
          (:`Update`
            (`MaterialInstanceDynamic.SetVectorParameterValue` _returnvalue "Color" _cookcolor)
            (set `self.cookRate` _cookfloat))
          (:`Finished`
            (set `self.isOvercooked` true)))))))

(event `self.Static Mesh.OnComponentEndOverlap`
  (params (OverlappedComponent :type "PrimitiveComponent Object Reference") (OtherActor :type "Actor Object Reference") (OtherComp :type "PrimitiveComponent Object Reference") (OtherBodyIndex :type Integer))
  (if (`KismetStringLibrary.EqualEqual_StrStr` "BP_Grill" (`KismetSystemLibrary.GetDisplayName` OtherActor))
    (goto _label :!via `Stop`)))

(fn `UserConstructionScript`
  (`parent.UserConstructionScript`))