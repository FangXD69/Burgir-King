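; BP_DownBun is the bottom burger bun that ingredients stack onto to assemble a hamburger.
; Its box overlap stops meat from cooking, then attaches any actor tagged Hamburger to a numbered mesh socket chosen by an incrementing counter, covering five slots.
; It enables player input on BeginPlay so mouse wheel up pitches the bun in fixed steps, with a debug print.
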(event `self.ReceiveBeginPlay`
  (`parent.ReceiveBeginPlay`)
  (`self.EnableInput` (`GameplayStatics.GetPlayerController` 0)))

(event `self.Box.OnComponentBeginOverlap`
  (params (OverlappedComponent :type "PrimitiveComponent Object Reference") (OtherActor :type "Actor Object Reference") (OtherComp :type "PrimitiveComponent Object Reference") (OtherBodyIndex :type Integer) (bFromSweep :type Boolean) (SweepResult :type "HitResult Structure (by ref)"))
  (if (`self.ActorHasTag` OtherActor "Meat")
    (bind _asbp_meat (cast `/Game/Blueprint/Food/New/BP_Meat` OtherActor))
    (set `/Game/Blueprint/Food/New/BP_Meat.canCook` false _asbp_meat))
  (if (`self.ActorHasTag` OtherActor "Hamburger")
    (bind _result (`/Engine/EditorBlueprintResources/StandardMacros.IncrementInt` (`self.numberOfComponent`))
      (:`  `
        (switch `int` _result
          (:`0`
            (set `self.upString` "Up0"))
          (:`1`
            (set `self.upString` "Up1"))
          (:`2`
            (set `self.upString` "Up2"))
          (:`3`
            (set `self.upString` "Up3"))
          (:`4`
            (set `self.upString` "Up4")))
        (`SceneComponent.K2_AttachToComponent` (`Actor.RootComponent` OtherActor) (`self.Static Mesh`) (`self.upString`) "SnapToTarget" "SnapToTarget" "KeepWorld" true)))))

(event `Key|MouseScrollUp`
  (params (Key :type "Key Structure"))
  (:`Pressed`
    (`KismetSystemLibrary.PrintString` "input")
    (`self.K2_AddActorLocalRotation` (`KismetMathLibrary.MakeRotator` 0.0 30.0))))

(fn `UserConstructionScript`
  (`parent.UserConstructionScript`))