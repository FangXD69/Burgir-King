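; BP_UnderBun is a bottom bun food item that serves as the base for stacking a hamburger.
; When an actor tagged "Hamburger" overlaps its Box, a counter selects one of five numbered sockets on the bun's StaticMesh.
; The actor's root then snaps to that socket's location and rotation, keeping world scale.
; Interact prints a pickup message and returns the bun's mesh.
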(event `self.Box.OnComponentBeginOverlap`
  (params (OverlappedComponent :type "PrimitiveComponent Object Reference") (OtherActor :type "Actor Object Reference") (OtherComp :type "PrimitiveComponent Object Reference") (OtherBodyIndex :type Integer) (bFromSweep :type Boolean) (SweepResult :type "HitResult Structure (by ref)"))
  (if (`self.ActorHasTag` OtherActor "Hamburger")
    (bind _result (`/Engine/EditorBlueprintResources/StandardMacros.IncrementInt` (`self.numberOfComponent`))
      (:`  `
        (switch `int` _result
          (:`0`
            (set `self.upString` "Up0"))
          (:`1`
            (set `self.upString` "Up1"))
          (:`2`
            (set `self.upString` "Up2"))
          (:`3`
            (set `self.upString` "Up3"))
          (:`4`
            (set `self.upString` "Up4")))
        (`SceneComponent.K2_AttachToComponent` (`Actor.RootComponent` OtherActor) (`self.StaticMesh`) (`self.upString`) "SnapToTarget" "SnapToTarget" "KeepWorld" true)))))

(fn `Interact`
  (returns (`Static Mesh` :type "StaticMesh Object Reference"))
  (`KismetSystemLibrary.PrintString` "Picked Up")
  (return (`StaticMeshComponent.StaticMesh` (`self.StaticMesh`))))

(fn `UserConstructionScript`)