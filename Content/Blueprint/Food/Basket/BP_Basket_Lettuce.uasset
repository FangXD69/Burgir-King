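; Lettuce basket that spawns a set number of ingredient actors and carries them while held.
; BeginPlay spawns items, snaps them to numbered Basket sockets, then detaches them in place.
; Hold reattaches items by array index, one lower than the spawn socket numbers, and Unhold detaches them.
; SetMovement forwards simulation to BP_Ingredient but returns after the first item, and overlap-exit removal is disconnected.
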(event `self.ReceiveBeginPlay`
  (for _index (range (`self.NumberOfIngredients`))
    (bind _returnvalue (`|SpawnActorFromClass` (`self.ItemClass`) (`KismetMathLibrary.MakeTransform` (`SceneComponent.K2_GetComponentLocation` (`self.ItemSpawnRoot`))) "Undefined" "MultiplyWithRoot" null null))
    (`self.Attach` _returnvalue (`KismetStringLibrary.Conv_StringToName` (`KismetStringLibrary.Conv_IntToString` (+ _index 1))))
    (`KismetArrayLibrary.Array_Add` (`self.Items`) _returnvalue))
  (for _array_element (`self.Items`)
    (`self.K2_DetachFromActor` _array_element "KeepWorld" "KeepWorld" "KeepWorld"))
  (set `self.canTest` true))

(event `self.Hold`
  (`KismetSystemLibrary.PrintString` "tut")
  (for (_array_element _array_index) (`self.Items`)
    (`self.Attach` _array_element (`KismetStringLibrary.Conv_StringToName` (`KismetStringLibrary.Conv_IntToString` _array_index)))))

(event `self.Unhold`
  (for _array_element (`self.Items`)
    (`self.K2_DetachFromActor` _array_element "KeepWorld" "KeepWorld" "KeepWorld")))

(event `self.Box.OnComponentEndOverlap`
  (params (OverlappedComponent :type "PrimitiveComponent Object Reference") (OtherActor :type "Actor Object Reference") (OtherComp :type "PrimitiveComponent Object Reference") (OtherBodyIndex :type Integer)))

(fn `UserConstructionScript`)