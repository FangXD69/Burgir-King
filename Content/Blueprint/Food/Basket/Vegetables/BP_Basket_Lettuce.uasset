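; Lettuce basket actor that spawns a set number of ingredient items and releases them when interacted with.
; On BeginPlay it spawns each item at the spawn root, snaps it to a numbered socket on the basket mesh and stores it.
; The InteractwithObjects event detaches all items in world space and destroys the basket.
; SetMovement forwards to BP_Ingredient but returns inside the loop, reaching only the first item.
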(event `self.ReceiveBeginPlay`
  (for _index (range (`self.NumberOfIngredients`))
    (bind _returnvalue (`|SpawnActorFromClass` (`self.ItemClass`) (`KismetMathLibrary.MakeTransform` (`SceneComponent.K2_GetComponentLocation` (`self.ItemSpawnRoot`))) "Undefined" "MultiplyWithRoot" null null))
    (`self.Attach` _returnvalue (`KismetStringLibrary.Conv_StringToName` (`KismetStringLibrary.Conv_IntToString` (+ _index 1))))
    (`KismetArrayLibrary.Array_Add` (`self.Items`) _returnvalue)))

(event `/Game/Blueprint/Player/BPI_Interact.InteractWithObjects`
  (for _array_element (`self.Items`)
    (`self.K2_DetachFromActor` _array_element "KeepWorld" "KeepWorld" "KeepWorld"))
  (`self.K2_DestroyActor`))

(fn `GetInteractState`
  (returns (InteractState :type Boolean))
  (return false))

(fn `Interact`
  (returns (`Static Mesh` :type "StaticMesh Object Reference"))
  (return null))

(fn `UserConstructionScript`)