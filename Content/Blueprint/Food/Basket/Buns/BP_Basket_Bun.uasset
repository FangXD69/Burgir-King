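; Bun basket actor that fills itself with top and bottom bun ingredients and releases them when interacted with.
; On BeginPlay it spawns alternating UpBun and DownBun actors, snaps each to the basket socket named by its index, and tracks them in Items.
; Interaction detaches the items in world space and destroys the basket, while SetMovement forwards the simulate flag to BP_Ingredient items.
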(event `self.ReceiveBeginPlay`
  (for _index (range 1 (+ (`self.NumberOfIngredients`) 1))
    (if (== (mod _index 2) 0)
      (`self.SpawnActor` (`self.DownBun`) _index)
      (else
        (`self.SpawnActor` (`self.UpBun`) _index)))))

(event `self.InteractWithObjects`
  (for _array_element (`self.Items`)
    (`self.K2_DetachFromActor` _array_element "KeepWorld" "KeepWorld" "KeepWorld"))
  (`self.K2_DestroyActor`))

(fn `GetInteractState`
  (returns (InteractState :type Boolean))
  (return false))

(fn `UserConstructionScript`)