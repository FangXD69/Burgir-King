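; BP_DownBun is the bottom bun that assembles a burger from food actors overlapping its box.
; Tagged ingredients snap to numbered mesh sockets in stack order, meat stops cooking, and a top bun attaches only once CanClose is set.
; The same overlap then records lettuce, cheese and meat types and counts for the order system.
; Player keys also pitch the bun, swap its mesh with an upward impulse, or destroy it.
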(event `self.ReceiveBeginPlay`
  (`parent.ReceiveBeginPlay`)
  (`self.EnableInput` (`GameplayStatics.GetPlayerController` 0)))

(event `self.ReceiveTick`
  (params (DeltaSeconds :type "Float (single-precision)")))

(event `self.Box.OnComponentBeginOverlap`
  (params (OverlappedComponent :type "PrimitiveComponent Object Reference") (OtherActor :type "Actor Object Reference") (OtherComp :type "PrimitiveComponent Object Reference") (OtherBodyIndex :type Integer) (bFromSweep :type Boolean) (SweepResult :type "HitResult Structure (by ref)"))
  (`|ExecutionSequence`
    (:`then_0`
      (if (`self.ActorHasTag` OtherActor "Hamburger")
        (if (`self.ActorHasTag` OtherActor "Meat")
          (bind _asbp_meat (cast `/Game/Blueprint/Food/BP_Meat` OtherActor))
          (set `/Game/Blueprint/Food/BP_Meat.canCook` false _asbp_meat))
        (if (`self.ActorHasTag` OtherActor "Down")
          _
          (elif (`self.ActorHasTag` OtherActor "UpBun")
            (if (`self.canClose`)
              (switch `int` (+ (`self.numberOfComponent`) 1) :!label _label
                (:`0`
                  (set `self.upString` "Up0"))
                (:`1`
                  (set `self.upString` "Up1"))
                (:`2`
                  (set `self.upString` "Up2"))
                (:`3`
                  (set `self.upString` "Up3"))
                (:`4`
                  (set `self.upString` "Up4")))
              (`SceneComponent.K2_AttachToComponent` (`Actor.RootComponent` OtherActor) (`self.Static Mesh`) (`self.upString`) "SnapToTarget" "SnapToTarget" "KeepWorld" true)
              (set `self.canClose` true)
              (`/Engine/EditorBlueprintResources/StandardMacros.IncrementInt` (`self.numberOfComponent`)))
            (else
              (goto _label))))))
    (:`then_1`
      (if (> (`self.numberOfComponent`) 0)
        ;[1 1 1] Burger order system
        (bind _asbp_lettuce (cast `/Game/Blueprint/Food/BP_Lettuce` OtherActor)
          (:`then`
            (set `self._LettuceType` (`/Game/Blueprint/Food/BP_Lettuce.LettuceType` _asbp_lettuce))
            (`/Engine/EditorBlueprintResources/StandardMacros.IncrementInt` (`self.LettuceCount`)))
          (:`CastFailed`
            (bind _asbp_cheese (cast `/Game/Blueprint/Food/BP_Cheese` OtherActor)
              (:`then`
                (set `self._CheseeType` (`/Game/Blueprint/Food/BP_Cheese.CheeseType` _asbp_cheese))
                (`/Engine/EditorBlueprintResources/StandardMacros.IncrementInt` (`self.CheeseCount`)))
              (:`CastFailed`
                (bind _asbp_meat_2 (cast `/Game/Blueprint/Food/BP_Meat` OtherActor))
                (set `self._MeatType` (`/Game/Blueprint/Food/BP_Meat.MeatType` _asbp_meat_2))
                (`/Engine/EditorBlueprintResources/StandardMacros.IncrementInt` (`self.MeatCount`))))))))))

(event `Key|MouseScrollUp`
  (params (Key :type "Key Structure"))
  (:`Pressed`
    (`KismetSystemLibrary.PrintString` "input")
    (`self.K2_AddActorLocalRotation` (`KismetMathLibrary.MakeRotator` 0.0 30.0))))

(event `Key|Q`
  (params (Key :type "Key Structure"))
  (bind _static_mesh (`self.Static Mesh`))
  (:`Pressed`
    (`StaticMeshComponent.SetStaticMesh` _static_mesh "/Game/Assets/Items/spacebux.spacebux")
    (`PrimitiveComponent.AddImpulse` _static_mesh (0.0 0.0 800.0) "None" false)))

(event `Key|E`
  (params (Key :type "Key Structure"))
  (:`Pressed`
    (`self.K2_DestroyActor`)))

(fn `UserConstructionScript`
  (`parent.UserConstructionScript`))