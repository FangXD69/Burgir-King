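; BP_OctopusArm is an octopus arm food item that cooks while overlapping BP_Grill, extending a parent class and setting its own MeatType.
; Grill overlap, matched by display name, plays a Timeline that drives a dynamic material's color and CookRate, flagging IsOvercooked when finished.
; Leaving the grill stops the Timeline.
; Tick uses paired DoOnce gates to start and stop a sizzling sound as grill contact changes.
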(event `self.ReceiveBeginPlay`
  (`parent.ReceiveBeginPlay`)
  (set `self.MeatType` "NewEnumerator6"))

(event `self.ReceiveTick`
  (params (DeltaSeconds :type "Float (single-precision)"))
  (bind _sound (`self.Sound`))
  (`parent.ReceiveTick` DeltaSeconds)
  (if (`self.canPlaySound`)
    (`/Engine/EditorBlueprintResources/StandardMacros.DoOnce` false :!label _label
      (:`Completed`
        (bind _returnvalue (`GameplayStatics.SpawnSound2D` "/Game/Assets/Sounds/SFX_Sizzling.SFX_Sizzling" 1.0 1.0 0.0 null))
        (set `self.Sound` _returnvalue)
        (goto _label_2 :!via `Reset`)))
    (else
      (`/Engine/EditorBlueprintResources/StandardMacros.DoOnce` false :!label _label_2
        (:`Completed`
          (`/Engine/EditorBlueprintResources/StandardMacros.IsValid` _sound
            (:`Is Valid`
              (`AudioComponent.Stop` _sound)
              (goto _label :!via `Reset`))))))))

(event `self.Static Mesh.OnComponentBeginOverlap`
  (params (OverlappedComponent :type "PrimitiveComponent Object Reference") (OtherActor :type "Actor Object Reference") (OtherComp :type "PrimitiveComponent Object Reference") (OtherBodyIndex :type Integer) (bFromSweep :type Boolean) (SweepResult :type "HitResult Structure (by ref)"))
  (if (`self.canCook`)
    (if (`KismetStringLibrary.EqualEqual_StrStr` "BP_Grill" (`KismetSystemLibrary.GetDisplayName` OtherActor))
      (set `self.canPlaySound` true)
      (if (not (`self.isOvercooked`))
        (bind _returnvalue (`PrimitiveComponent.CreateDynamicMaterialInstance` (`self.Static Mesh`) 0 "/Game/Assets/Food/meat.meat" "None"))
        (bind (_direction _cookcolor _cookfloat) (`Timeline|Timeline` :!label _label_3)
          (:`Update`
            (`MaterialInstanceDynamic.SetVectorParameterValue` _returnvalue "Color" _cookcolor)
            (set `self.cookRate` _cookfloat))
          (:`Finished`
            (set `self.isOvercooked` true)))))))

(event `self.Static Mesh.OnComponentEndOverlap`
  (params (OverlappedComponent :type "PrimitiveComponent Object Reference") (OtherActor :type "Actor Object Reference") (OtherComp :type "PrimitiveComponent Object Reference") (OtherBodyIndex :type Integer))
  (if (`KismetStringLibrary.EqualEqual_StrStr` "BP_Grill" (`KismetSystemLibrary.GetDisplayName` OtherActor))
    (set `self.canPlaySound` false)
    (goto _label_3 :!via `Stop`)))

(fn `UserConstructionScript`
  (`parent.UserConstructionScript`))