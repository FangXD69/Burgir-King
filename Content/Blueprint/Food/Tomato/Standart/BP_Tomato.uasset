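; Tomato food item that is cut into slices through a hold interaction.
; On BeginPlay it caches its hold-key widget, then shows or hides it every Tick based on CanShowWidget.
; The ProgressHold event feeds hold progress into the widget's progress bar and prints a debug string.
; At full progress it spawns BP_TomatoSlice actors at its location and destroys itself.
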(event `self.ReceiveBeginPlay`
  (`parent.ReceiveBeginPlay`)
  (bind _aswb_hold_key (cast `/Game/Blueprint/Food/Basket/WB_HoldKey` (`WidgetComponent.GetWidget` (`self.Widget`))))
  (set `self.HoldWidget` _aswb_hold_key))

(event `self.ReceiveTick`
  (params (DeltaSeconds :type "Float (single-precision)"))
  (`parent.ReceiveTick` DeltaSeconds)
  (if (`self.canShowWidget`)
    (`Widget.SetVisibility` (`self.HoldWidget`) "Visible")
    (else
      (`Widget.SetVisibility` (`self.HoldWidget`) "Hidden"))))

(event `/Game/Blueprint/Player/BPI_Hold.ProgressHold`
  (params (Progress :type "Float (double-precision)"))
  (`KismetSystemLibrary.PrintString` "kesiliyor")
  (`ProgressBar.SetPercent` (`/Game/Blueprint/Food/Basket/WB_HoldKey.ProgressBar` (`self.HoldWidget`)) Progress)
  (if (== Progress 1.0)
    (for _ (range 3)
      (`|SpawnActorFromClass` "/Game/Blueprint/Food/Tomato/Standart/BP_TomatoSlice.BP_TomatoSlice_C" (`KismetMathLibrary.MakeTransform` (`self.K2_GetActorLocation`)) "Undefined" "MultiplyWithRoot" null null))
    (`self.K2_DestroyActor`)))

(fn `UserConstructionScript`
  (`parent.UserConstructionScript`))