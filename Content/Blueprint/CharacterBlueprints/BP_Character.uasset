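; Restaurant customer character that orders a menu item, walks to a table, eats a burger and leaves.
; ConstructCharacter receives the locations and order; MoveOrder starts the AI walk to the order point.
; Tick watches state flags through DoOnce gates to fill the order widget, then move to the table.
; EatBurger spawns payment only if happy, then sends the customer to exit and destruction; SitOrGetUp attaches the mesh to a chair socket or detaches it.
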(event `self.ReceiveBeginPlay`)

(event `self.ReceiveTick`
  (params (DeltaSeconds :type "Float (single-precision)"))
  (`|ExecutionSequence`
    (:`then_0`
      (if (`self.OnOrderPoint`)
        (`/Engine/EditorBlueprintResources/StandardMacros.DoOnce` false
          (:`Completed`
            (bind _aswb_customer_order (cast `/Game/Blueprint/Systems/MenuOrder/OrderWidget/CustomerSide/WB_CustomerOrder` (`WidgetComponent.GetWidget` (`self.W_Order`))))
            (set `/Game/Blueprint/Systems/MenuOrder/OrderWidget/CustomerSide/WB_CustomerOrder.OrderText` (`KismetTextLibrary.Conv_StringToText` (`self.FoodCustomerWants`)) _aswb_customer_order)))))
    (:`then_1`
      (if (`self.GoingTable`)
        (`/Engine/EditorBlueprintResources/StandardMacros.DoOnce` false
          (:`Completed`
            (`|AIMoveTo` self (`self.MyTableLoc`) null 10.0
              (:`then`
                (`SceneComponent.SetVisibility` (`self.W_Order`) false false))
              (:`OnSuccess`
                (set `self.arrivedTable` true)))))))))

(event `/Game/Blueprint/Systems/MenuOrder/BPI_OrderPoint.MoveOrder`
  (if (not (`self.GoingTable`))
    (`|AIMoveTo` self (`self.OrderPoint`) null)))

(event `GoOutEvent`
  (if (`self.IsHappy`)
    (`KismetSystemLibrary.PrintString` "NiiceBURGER!!!!!!! SEE YAAAAAAA")
    (else
      (`KismetSystemLibrary.PrintString` "I didn't like the burger. Fuck You!" true true (struct :`R` 0.851189 :`G` 1.0 :`A` 1.0))))
  (`|AIMoveTo` self (`self.ExitPoint`) null 10.0
    (:`OnSuccess`
      (`self.K2_DestroyActor`))))

(fn `ConstructCharacter`
  (params (MyTableLoc :type "Vector Structure") (OrderPoint :type "Vector Structure") (ExitPoint :type "Vector Structure") (MenuName :type String))
  (set `self.MyTableLoc` MyTableLoc)
  (set `self.OrderPoint` OrderPoint)
  (set `self.ExitPoint` ExitPoint)
  (set `self.FoodCustomerWants` MenuName))

(fn `EatBurger`
  (params (Burger :type "/Game/Blueprint/Food/Breads/BP_DownBun Object Reference") (` MoneyAmount` :type "Float (double-precision)"))
  (if (`self.IsHappy`)
    (`/Game/Blueprint/Food/Breads/BP_DownBun.Destroy Itself` Burger)
    (bind _returnvalue (`|SpawnActorFromClass` "/Game/Blueprint/Systems/MenuOrder/BP_SpaceBux.BP_SpaceBux_C" (`KismetMathLibrary.MakeTransform` (`SceneComponent.K2_GetComponentLocation` (`self.MoneySpawnLocation`))) "Undefined" "MultiplyWithRoot" null null))
    (set `/Game/Blueprint/Systems/MenuOrder/BP_SpaceBux. MoneyAmount` ` MoneyAmount` _returnvalue)
    (`self.GoOutEvent`)
    (else
      (`self.GoOutEvent`))))

(fn `SitOrGetUp`
  (params (Sit :type Boolean) (Chair :type "StaticMeshComponent Object Reference") (AddOffset :type "Float (double-precision)"))
  (`KismetSystemLibrary.PrintString` "ÇALIŞIYOR \n")
  (if Sit
    (`SceneComponent.K2_AttachToComponent` (`self.Mesh`) Chair "SitPoint" "SnapToTarget" "KeepRelative" "KeepWorld" true)
    (else
      (`self.K2_DetachFromActor` self "KeepRelative" "KeepRelative" "KeepWorld")
      (`SceneComponent.K2_AddWorldOffset` (`self.Mesh`) (`KismetMathLibrary.MakeVector` AddOffset) false false))))

(fn `UserConstructionScript`)