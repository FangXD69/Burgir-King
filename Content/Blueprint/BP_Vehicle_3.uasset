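; BP_Vehicle_3 is a looping vehicle actor that repeatedly moves its Vehicle component along a path, starting five seconds after BeginPlay.
; Each cycle snaps the vehicle to the Arrival2 location, then a timeline lerps it from a hard-coded local position to Arrival1 without sweeping.
; The loop re-triggers through a Delay on the timeline's Update output rather than on Finished.
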(event `self.ReceiveBeginPlay`
  (`KismetSystemLibrary.Delay` 5.0)
  (`self.CarCycle_1`))

(event `CarCycle_1`
  (`KismetSystemLibrary.Delay` 0.2)
  (`self.carcycle_2`)
  (`KismetSystemLibrary.Delay` 1.0)
  (bind (_direction _newtrack_0) (`Timeline|Timeline` :!via `PlayFromStart`)
    (:`Update`
      (`SceneComponent.K2_SetRelativeLocation` (`self.vehicle`) (`KismetMathLibrary.VLerp` (0.0 450.0 -100.0) (`SceneComponent.RelativeLocation` (`self.arrival_1`)) _newtrack_0) false false)
      (`KismetSystemLibrary.Delay` 4.0)
      (`self.CarCycle_1`))))

(event `carcycle_2`
  (`SceneComponent.K2_SetRelativeLocation` (`self.vehicle`) (`SceneComponent.RelativeLocation` (`self.arrival_2`)) false false))

(fn `UserConstructionScript`)