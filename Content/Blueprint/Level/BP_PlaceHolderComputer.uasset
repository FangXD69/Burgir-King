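; Placeholder computer actor that shows an ingredient order UI while the player pawn stands in its overlap volume.
; On BeginPlay it creates the WB_IngredientOrder widget, passes itself to it, and binds to the BP_Status game state's money-changed event to mirror Money into BankAccount.
; Cube overlap begin and end call SetOrderWidget, which adds or removes the widget and switches mouse cursor and input mode.
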(event `self.ReceiveBeginPlay`
  (bind _returnvalue (`|CreateWidget` "/Game/Blueprint/Systems/IngredientOrder/WB_IngredientOrder.WB_IngredientOrder_C" (`GameplayStatics.GetPlayerController` 0)))
  (bind _output_get (set `self.OrderWB` _returnvalue))
  (set `/Game/Blueprint/Systems/IngredientOrder/WB_IngredientOrder.Computer` self _output_get)
  (bind _asbp_status (cast `/Game/Blueprint/Systems/BP_Status` (`GameplayStatics.GetGameState`)))
  (bind _output_get_2 (set `self.Status` _asbp_status))
  (add `/Game/Blueprint/Systems/BP_Status.DP_OnMoneyChanged` _output_get_2 (delegate `OnMoneyChanged`)))

(event `OnMoneyChanged`
  (params (AmountOfMoneyChanged :type Integer) (Money :type Integer))
  (set `self.BankAccount` Money))

(event `self.Cube.OnComponentBeginOverlap`
  (params (OverlappedComponent :type "PrimitiveComponent Object Reference") (OtherActor :type "Actor Object Reference") (OtherComp :type "PrimitiveComponent Object Reference") (OtherBodyIndex :type Integer) (bFromSweep :type Boolean) (SweepResult :type "HitResult Structure (by ref)"))
  (if (== OtherActor (`Controller.K2_GetPawn` (`GameplayStatics.GetPlayerController` 0)))
    (bind _asbp_player (cast `/Game/Blueprint/Player/BP_Player` OtherActor))
    (set `self.Player` _asbp_player)
    (`self.Set Order Widget` true)))

(event `self.Cube.OnComponentEndOverlap`
  (params (OverlappedComponent :type "PrimitiveComponent Object Reference") (OtherActor :type "Actor Object Reference") (OtherComp :type "PrimitiveComponent Object Reference") (OtherBodyIndex :type Integer))
  (if (== OtherActor (`Controller.K2_GetPawn` (`GameplayStatics.GetPlayerController` 0)))
    (`self.Set Order Widget` false)))

(fn `Set Order Widget`
  (params (Open :type Boolean))
  (bind _returnvalue (`GameplayStatics.GetPlayerController` 0))
  (if Open
    (`UserWidget.AddToViewport` (`self.OrderWB`) 0)
    (set `PlayerController.bShowMouseCursor` true _returnvalue)
    (`WidgetBlueprintLibrary.SetInputMode_GameAndUIEx` _returnvalue (`self.OrderWB`) "DoNotLock" false)
    (else
      (`Widget.RemoveFromParent` (`self.OrderWB`))
      (set `PlayerController.bShowMouseCursor` false _returnvalue)
      (`WidgetBlueprintLibrary.SetInputMode_GameOnly` _returnvalue))))

(fn `UserConstructionScript`)