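; BP_Table is a restaurant table that scores a served burger against the customer's order and pays out money.
; One box stores an overlapping BP_DownBun as the burger; the other, after a delay, loads an arrived customer's order from the menu DataTable.
; That same delayed overlap runs Compare on cheese, lettuce and meat, docking price for wrong types or counts.
; The truncated price goes to BP_Status once; meat doneness is read but never compared.
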(event `self.ReceiveBeginPlay`
  (bind _asbp_status (cast `/Game/Blueprint/Systems/BP_Status` (`GameplayStatics.GetGameState`)))
  (set `self.GameState` _asbp_status))

(event `self.Box.OnComponentBeginOverlap`
  (params (OverlappedComponent :type "PrimitiveComponent Object Reference") (OtherActor :type "Actor Object Reference") (OtherComp :type "PrimitiveComponent Object Reference") (OtherBodyIndex :type Integer) (bFromSweep :type Boolean) (SweepResult :type "HitResult Structure (by ref)"))
  (bind _burger (`self.Burger`))
  (bind _burger_2 (`self.Burger`))
  (bind _burger_3 (`self.Burger`))
  (bind _returnvalue (`KismetStringLibrary.Conv_StringToName` (`/Game/Blueprint/CharacterBlueprints/BP_Character.FoodCustomerWants` (`self.Customer`))))
  (`KismetSystemLibrary.Delay` 1.0)
  (`|ExecutionSequence`
    (:`then_0`
      (bind _asbp_character (cast `/Game/Blueprint/CharacterBlueprints/BP_Character` OtherActor))
      (set `self.Customer` _asbp_character)
      (if (`/Game/Blueprint/CharacterBlueprints/BP_Character.arrivedTable` _asbp_character)
        (`KismetSystemLibrary.PrintString` (`KismetStringLibrary.Conv_NameToString` _returnvalue))
        (bind _returnvalue_2 (`|GetDataTableRow` "/Game/Blueprint/Systems/MenuOrder/MenuDataTable.MenuDataTable" _returnvalue)
          (:`then`
            (bind (_menuname _bun _cheese _cheesecount _meat _meatdoneness _meatcount _lettuce _lettucecount _menuprice) (break `/Game/Blueprint/Systems/MenuOrder/OrderStructure` _returnvalue_2))
            (set `self.MenuCheeseType` _cheese)
            (set `self.MenuCheeseCount` _cheesecount)
            (set `self.MenuMeatType` _meat)
            (set `self.MeatDoneness` _meatdoneness)
            (set `self.MenuMeatCount` _meatcount)
            (set `self.MenuLettuceType` _lettuce)
            (set `self.MenuLettuceCount` _lettucecount)
            (bind _output_get (set `self.MenuPrice` _menuprice))
            (`KismetSystemLibrary.PrintString` (`KismetStringLibrary.Conv_DoubleToString` _output_get))))))
    (:`then_2`
      (`/Engine/EditorBlueprintResources/StandardMacros.IsValid` (`self.Burger`)
        (:`Is Valid`
          (if (`self.CanCalculate`)
            ;[1 1 1] CompareCheese
            (`self.Compare` (`/Game/Blueprint/Food/BP_DownBun._CheseeType` _burger_2) (`/Game/Blueprint/Food/BP_DownBun.CheeseCount` _burger_2) (`self.MenuCheeseType`) (`self.MenuCheeseCount`))
            ;[1 1 1] CompareLettuce
            (`self.Compare` (`/Game/Blueprint/Food/BP_DownBun._LettuceType` _burger) (`/Game/Blueprint/Food/BP_DownBun.LettuceCount` _burger) (`self.MenuLettuceType`) (`self.MenuLettuceCount`))
            ;[1 1 1] Comment
            (`self.Compare` (`/Game/Blueprint/Food/BP_DownBun._MeatType` _burger_3) (`/Game/Blueprint/Food/BP_DownBun.MeatCount` _burger_3) (`self.MenuMeatType`) (`self.MenuMeatCount`))
            (`/Game/Blueprint/Systems/BP_Status.DP_OnMoneyChanged` (`self.GameState`) (`KismetMathLibrary.FTrunc` (`self.MenuPrice`)))
            (set `self.CanCalculate` false)))
        (:`Is Not Valid`
          (`KismetSystemLibrary.PrintString` "Burger NOT VALID" true true (struct :`R` 1.0 :`B` 0.09376 :`A` 1.0)))))
    (:`then_3`
      (`KismetSystemLibrary.PrintString` (`KismetStringLibrary.Concat_StrStr` "Menu Fiyat: " (`KismetStringLibrary.Conv_DoubleToString` (`self.MenuPrice`)))))))

(event `self.ReceiveTick`
  (params (DeltaSeconds :type "Float (single-precision)"))
  (if (not (`self.CanCalculate`))
    (`KismetSystemLibrary.Delay` 0.5)
    (`KismetSystemLibrary.PrintString` (`KismetStringLibrary.Concat_StrStr` "Menu price:  " (`KismetStringLibrary.Conv_DoubleToString` (`self.MenuPrice`))) true true (struct :`R` 0.889895 :`B` 1.0 :`A` 1.0))))

(event `self.Box1.OnComponentBeginOverlap`
  (params (OverlappedComponent :type "PrimitiveComponent Object Reference") (OtherActor :type "Actor Object Reference") (OtherComp :type "PrimitiveComponent Object Reference") (OtherBodyIndex :type Integer) (bFromSweep :type Boolean) (SweepResult :type "HitResult Structure (by ref)"))
  (bind _asbp_down_bun (cast `/Game/Blueprint/Food/BP_DownBun` OtherActor))
  (set `self.Burger` _asbp_down_bun)
  (`KismetSystemLibrary.PrintString` "BurgerValid" true true (struct :`R` 0.024024 :`G` 1.0 :`A` 1.0)))

(fn `UserConstructionScript`)