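; Front desk computer that takes a customer's order when the player interacts with it.
; With a valid Customer, Order sets its GoingTable flag, swaps the screen slot to the Rocketburger material for a second, then reruns Construct.
; Construct creates a dynamic screen material but immediately puts the menu material on that slot.
; Helper functions handle the computer widget and cursor input mode, though the event graph never calls them.
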(event `self.ReceiveTick`
  (params (DeltaSeconds :type "Float (single-precision)")))

(event `self.ReceiveBeginPlay`
  (`self.Construct`))

(event `Construct`
  (bind _returnvalue (`PrimitiveComponent.CreateDynamicMaterialInstance` (`self.StaticMesh`) 4 "/Game/Assets/InteractableStuff/M_FrontDeskScreen.M_FrontDeskScreen" "None"))
  (set `self.ScreenMaterial` _returnvalue)
  (`PrimitiveComponent.SetMaterial` (`self.StaticMesh`) 4 "/Game/Blueprint/PC/M_Menu1.M_Menu1"))

(event `Order`
  (`KismetSystemLibrary.PrintString` "pressede")
  (bind _customer (`self.Customer`)
    (:`then`
      (`KismetSystemLibrary.PrintString` "Valdi" true true (struct :`R` 1.0 :`G` 0.199848 :`A` 1.0))
      (set `/Game/Blueprint/CharacterBlueprints/BP_Character.GoingTable` true _customer)
      (`PrimitiveComponent.SetMaterial` (`self.StaticMesh`) 4 "/Game/Blueprint/PC/M_Rocketburger.M_Rocketburger")
      (`KismetSystemLibrary.Delay` 1.0)
      (`MaterialInstanceDynamic.SetVectorParameterValue` (`self.ScreenMaterial`) "Screen" (struct :`R` 1.0 :`B` 0.041833 :`A` 1.0))
      (`self.Construct`))
    (:`else`)))

(event `/Game/Blueprint/Player/BPI_Interact.InteractWithObjects`
  (`self.Order`))

(fn `GetInteractState`
  (returns (InteractState :type Boolean))
  (return (`self.Interact State`)))

(fn `RecreateWidget`
  (`Widget.RemoveFromParent` (`self.ComputerWidget`))
  (set `self.ComputerWidget` null)
  (bind _returnvalue (`|CreateWidget` "/Game/Blueprint/Systems/MenuOrder/OrderWidget/CustomerSide/WB_CustomerComputer.WB_CustomerComputer_C"))
  (set `self.ComputerWidget` _returnvalue)
  (return))

(fn `SetUI`
  (params (Condition :type Boolean))
  (bind _returnvalue (`GameplayStatics.GetPlayerController` 0))
  (bind _computerwidget (`self.ComputerWidget`))
  (if Condition
    (`WidgetBlueprintLibrary.SetInputMode_GameAndUIEx` _returnvalue _computerwidget)
    (set `PlayerController.bShowMouseCursor` true _returnvalue)
    (else
      (`Widget.RemoveFromParent` _computerwidget)
      (set `PlayerController.bShowMouseCursor` false _returnvalue)
      (`WidgetBlueprintLibrary.SetInputMode_GameOnly` _returnvalue))))

(fn `UserConstructionScript`
  (`parent.UserConstructionScript`))