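; BP_SpaceBux is a money pickup actor that the player collects by interacting with it.
; On BeginPlay it casts the game state to BP_Status and caches the reference.
; InteractwithObjects passes its MoneyAmount, truncated to an integer, to CallDPOnMoneyChanged on that game state, then destroys the actor.
; GetInteractState always returns false.
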(event `self.ReceiveBeginPlay`
  (bind _asbp_status (cast `/Game/Blueprint/Systems/BP_Status` (`GameplayStatics.GetGameState`)))
  (set `self.GameState` _asbp_status))

(event `/Game/Blueprint/Player/BPI_Interact.InteractWithObjects`
  (`/Game/Blueprint/Systems/BP_Status.DP_OnMoneyChanged` (`self.GameState`) (`KismetMathLibrary.FTrunc` (`self. MoneyAmount`)))
  (`self.K2_DestroyActor`))

(fn `GetInteractState`
  (returns (InteractState :type Boolean))
  (return false))

(fn `UserConstructionScript`)