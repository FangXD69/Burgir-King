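; Customer system actor that spawns restaurant customers on the server and sends them to order.
; HourIncreased calls Order, which spawns a random customer class, then re-calls itself after a delay.
; AIMoveTo walks each customer to an order point, then passes it a random menu DataTable row, table and exit at spawn.
; Points are actor-local; assigned tables leave the Tables pool, while TableClean appends to OrderPoints.
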(event `self.ReceiveBeginPlay`)

(event `Order`
  (`/Engine/EditorBlueprintResources/ActorMacros.Switch Has Authority`
    (:`Authority`
      (bind _outrownames (`DataTableFunctionLibrary.GetDataTableRowNames` "/Game/Blueprint/Systems/MenuOrder/MenuDataTable.MenuDataTable"))
      (set `self.Orders` _outrownames)
      (for _index (range 1)
        (bind _returnvalue (`|SpawnActorFromClass` (`KismetArrayLibrary.Array_Random` (`self.Customers`)) (`KismetMathLibrary.MakeTransform` (`self.LocalToWorldPos` (`self.SpawnPoint`))) "Undefined" "MultiplyWithRoot" null null))
        (`KismetSystemLibrary.PrintString` (`KismetSystemLibrary.GetDisplayName` _returnvalue))
        (`/Engine/EditorBlueprintResources/StandardMacros.IsValid` _returnvalue
          (:`Is Valid`
            (`self.SetCharacterMove` _returnvalue _index))))
      (`KismetSystemLibrary.PrintString` "SPAWNED")
      (`KismetSystemLibrary.Delay` 15.0)
      (`self.Order`))))

(event `/Game/Blueprint/Systems/DayCycle/BPI_MessageToCustomerSystem.HourIncreased`
  (`self.Order`))

(event `/Game/Blueprint/Systems/DayCycle/BPI_MessageToCustomerSystem.TableClean`
  (params (TableLoc :type "Vector Structure"))
  (`KismetArrayLibrary.Array_Add` (`self.OrderPoints`) TableLoc))

(event `SetCharacterMove`
  (params (`Actor ` :type "Actor Object Reference") (Index :type Integer))
  (bind _asbp_character (cast `/Game/Blueprint/CharacterBlueprints/BP_Character` `Actor `))
  (`|AIMoveTo` _asbp_character (`self.Arr_LocalToWorldPos` (`self.OrderPoints`) Index) null
    (:`then`
      (`/Game/Blueprint/CharacterBlueprints/BP_Character.ConstructCharacter` _asbp_character (`self.CreateTableLoc`) (`self.LocalToWorldPos` (`self.OrderPoint`)) (`self.LocalToWorldPos` (`self.SpawnPoint`)) (`KismetStringLibrary.Conv_NameToString` (`KismetArrayLibrary.Array_Random` (`self.Orders`))))
      (`/Engine/EditorBlueprintResources/StandardMacros.IncrementInt` (`self.Index`)))))

(fn `CreateTableLoc`
  (returns (TableToGo :type "Vector Structure"))
  (bind _output_get (set `self.DumpTable` (`KismetArrayLibrary.Array_Random` (`self.Tables`))))
  (if (`KismetMathLibrary.Vector_IsZero` _output_get)
    (bind _output_get_2 (set `self.TableToGo` (`self.SpawnPoint`)))
    (`KismetSystemLibrary.PrintString` (`KismetStringLibrary.Concat_StrStr` "zero vector: " (`KismetStringLibrary.Conv_VectorToString` _output_get_2)))
    (return (`self.LocalToWorldPos` _output_get_2))
    (else
      (bind _output_get_3 (set `self.TableToGo` (`self.DumpTable`)))
      (`KismetSystemLibrary.PrintString` (`KismetStringLibrary.Concat_StrStr` "noprmal vector: " (`KismetStringLibrary.Conv_VectorToString` _output_get_3)))
      (`KismetArrayLibrary.Array_RemoveItem` (`self.Tables`) (`self.DumpTable`))
      (return (`self.LocalToWorldPos` _output_get_3)))))

(fn `UserConstructionScript`)