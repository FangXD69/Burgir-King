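; Customer system actor that spawns the restaurant's customers at BeginPlay and gives each a food order.
; It spawns every class in Customers at SpawnPoint and sends each by AI MoveTo to its indexed OrderPoints entry, both converted from actor-local positions.
; The move-completion branch sets FoodName from the OrderDataTable row names using an incrementing Index, then caches the character's WB_CustomerOrder widget.
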(event `self.ReceiveBeginPlay`
  (bind _outrownames (`DataTableFunctionLibrary.GetDataTableRowNames` "/Game/Blueprint/Systems/OrderSystem/OrderDataTable.OrderDataTable"))
  (set `self.Orders` _outrownames)
  (for (_array_element _array_index) (`self.Customers`)
    (bind _returnvalue (`|SpawnActorFromClass` _array_element (`KismetMathLibrary.MakeTransform` (`self.LocalToWorldPos` (`self.SpawnPoint`))) "Undefined" "MultiplyWithRoot" null null))
    (bind _asbp_character (cast `/Game/Blueprint/CharacterBlueprints/BP_Character` _returnvalue))
    (`|AIMoveTo` _asbp_character (`self.Arr_LocalToWorldPos` (`self.OrderPoints`) _array_index) null
      (:`then`
        (set `/Game/Blueprint/CharacterBlueprints/BP_Character.FoodName` (`KismetStringLibrary.Conv_NameToString` (`|GetArrayItem` (`self.Orders`) (`self.Index`))) _asbp_character)
        (bind _aswb_customer_order (cast `/Game/Blueprint/Systems/OrderSystem/OrderWidget/WB_CustomerOrder` (`WidgetComponent.GetWidget` (`/Game/Blueprint/CharacterBlueprints/BP_Character.W_Order` _asbp_character))))
        (set `self.Widget` _aswb_customer_order)
        (`/Engine/EditorBlueprintResources/StandardMacros.IncrementInt` (`self.Index`))))))

(fn `UserConstructionScript`)