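; BP_GravityAnomaly is a gravity anomaly that makes BP_Ingredient actors float until an actor overlaps it.
; A Tick-driven seconds counter sets CanGetIngredients at six seconds, letting a DoOnce cache all ingredient actors in Items.
; The Enable event calls SetGravity to switch off mesh gravity on the cached items and push them upward with an impulse.
; An overlap while gravity is off restores it.
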(event `self.ReceiveTick`
  (params (DeltaSeconds :type "Float (single-precision)"))
  (`|ExecutionSequence`
    (:`then_0`
      (if (`self.canGetIngredients`)
        (`/Engine/EditorBlueprintResources/StandardMacros.DoOnce` false
          (:`Completed`
            (bind _outactors (`GameplayStatics.GetAllActorsOfClass` "/Game/Blueprint/Food/BP_Ingredient.BP_Ingredient_C"))
            (set `self.Items` _outactors)))))
    (:`then_1`
      (`KismetSystemLibrary.Delay` 1.0)
      (bind _result (`/Engine/EditorBlueprintResources/StandardMacros.IncrementInt` (`self.Second`))
        (:`  `
          (if (and (== 6 (`self.Second`)) (not (`self.gravityIsOff`)))
            (set `self.Second` 0)
            (set `self.canGetIngredients` true)
            (`KismetSystemLibrary.Delay` 0.2)))))))

(event `/Game/Blueprint/Systems/BPI_Gravity.Enable`
  (`self.Set Gravity` false)
  (set `self.canGetIngredients` false))

(event `self.ReceiveActorBeginOverlap`
  (params (OtherActor :type "Actor Object Reference"))
  (if (`self.gravityIsOff`)
    (`self.Set Gravity` true)))

(fn `Set Gravity`
  (params (SetGravity :type Boolean))
  (if (not SetGravity)
    (for _array_element (`self.Items`)
      (bind _static_mesh (`/Game/Blueprint/Food/BP_Ingredient.Static Mesh` _array_element))
      (`PrimitiveComponent.SetEnableGravity` _static_mesh false)
      (`PrimitiveComponent.AddImpulse` _static_mesh (0.0 0.0 500.0) "None" false)
      (`KismetSystemLibrary.PrintString` "Yer çekimi kapandı")
      (set `self.gravityIsOff` true))
    (else
      (for _array_element_2 (`self.Items`)
        (`PrimitiveComponent.SetEnableGravity` (`/Game/Blueprint/Food/BP_Ingredient.Static Mesh` _array_element_2) true)
        (`KismetSystemLibrary.PrintString` "Yer çekimi Açıldı")
        (set `self.gravityIsOff` false)))))

(fn `UserConstructionScript`)