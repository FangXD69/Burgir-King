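; BP_DayCycleControlPanel is an interactable control panel that starts or ends the in-game day.
; It finds and caches the BP_ClockManager on BeginPlay.
; On interaction it calls the manager's StartDay when the current hour is exactly 9 or EndDay when it is exactly 23, and otherwise does nothing.
; GetInteractState always returns false.
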(event `self.ReceiveBeginPlay`
  (bind _returnvalue (`GameplayStatics.GetActorOfClass` "/Game/Blueprint/Systems/DayCycle/BP_ClockManager.BP_ClockManager_C"))
  (set `self.ClockManager` _returnvalue))

(event `/Game/Blueprint/Player/BPI_Interact.InteractWithObjects`
  (bind _clockmanager (`self.ClockManager`))
  (bind _currenthour (`/Game/Blueprint/Systems/DayCycle/BP_ClockManager.CurrentHour` _clockmanager))
  (if (== _currenthour 9)
    (`/Game/Blueprint/Systems/DayCycle/BP_ClockManager.StartDay` _clockmanager)
    (elif (== _currenthour 23)
      (`/Game/Blueprint/Systems/DayCycle/BP_ClockManager.EndDay` _clockmanager))))

(fn `GetInteractState`
  (returns (InteractState :type Boolean))
  (return false))

(fn `UserConstructionScript`)