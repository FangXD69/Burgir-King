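; Clock manager actor that runs the in-game business day and shows the time on the player UI.
; While active, Tick converts real time into game minutes, updates the clock text and notifies BP_CustomerSystem on each hour change.
; StartDay starts the clock and records the bank balance from BP_Status.
; EndDay stops it and shows an end-of-day widget with profit and menus sold; the midnight check in Tick is empty.
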(event `self.ReceiveBeginPlay`
  (bind _returnvalue (`|CreateWidget` "/Game/Blueprint/Systems/DayCycle/WB_PlayerUI.WB_PlayerUI_C"))
  (bind _output_get (set `self.ClockWidget` _returnvalue))
  (`self.InitializeClockWidget` _output_get)
  (bind _asbp_status (cast `/Game/Blueprint/Systems/BP_Status` (`GameplayStatics.GetGameState`)))
  (set `self.GameState` _asbp_status)
  (bind _returnvalue_2 (`GameplayStatics.GetActorOfClass` "/Game/Blueprint/Systems/MenuOrder/BP_CustomerSystem.BP_CustomerSystem_C"))
  (set `self.CustomerSystem` _returnvalue_2))

(event `self.ReceiveTick`
  (params (DeltaSeconds :type "Float (single-precision)"))
  (if (`self.IsClockActive`)
    (set `self.TotalGameMinutes` (+ (* DeltaSeconds (`self.MinutesPerSecond`)) (`self.TotalGameMinutes`)))
    (set `self.DumpHour` (`self.CurrentHour`))
    (bind _output_get (set `self.CurrentHour` (+ 9 (`KismetMathLibrary.FFloor` (/ (`self.TotalGameMinutes`) 60.0)))))
    (if (not (== _output_get (`self.DumpHour`)))
      (message `/Game/Blueprint/Systems/DayCycle/BPI_MessageToCustomerSystem.HourIncreased` (`self.CustomerSystem`))
      (set `self.DumpHour` (`self.CurrentHour`)))
    (set `self.CurrentMinute` (`KismetMathLibrary.FTrunc` (`KismetMathLibrary.FMod` (`self.TotalGameMinutes`) 60.0)))
    (`/Engine/EditorBlueprintResources/StandardMacros.IsValid` (`self.ClockWidget`)
      (:`Is Valid`
        (`self.UpdateClockText`)
        (if (== (`self.CurrentHour`) 24)
          _)))))

(event `UpdateClockText`
  (set `TextBlock.Text` (`|FormatText` "{HH}:{MM}" (`KismetTextLibrary.Conv_IntToText` (`self.CurrentHour`) false true 2 2) (`KismetTextLibrary.Conv_IntToText` (`self.CurrentMinute`) false true 2 2)) (`/Game/Blueprint/Systems/DayCycle/WB_PlayerUI.ClockText` (`self.ClockWidget`))))

(fn `CalculateProfit`
  (returns (Profit :type Integer))
  (bind _gamestate (`self.GameState`))
  (return (- (`/Game/Blueprint/Systems/BP_Status.BankAccount` _gamestate) (`/Game/Blueprint/Systems/BP_Status.DayStartBankPrice` _gamestate))))

(fn `ConstructWidget`
  (params (`End Widget` :type "/Game/Blueprint/Systems/DayCycle/WB_EndDay Object Reference"))
  (set `TextBlock.Text` (`KismetTextLibrary.Conv_StringToText` (`KismetStringLibrary.Concat_StrStr` "$" (`KismetStringLibrary.Conv_IntToString` (`self.CalculateProfit`)))) (`/Game/Blueprint/Systems/DayCycle/WB_EndDay.Profit` `End Widget`))
  (set `TextBlock.Text` (`KismetTextLibrary.Conv_IntToText` (`/Game/Blueprint/Systems/BP_Status.MenusSold` (`self.GameState`))) (`/Game/Blueprint/Systems/DayCycle/WB_EndDay.MenusSold` `End Widget`)))

(fn `EndDay`
  (locals (DayEndWidget :type "/Game/Blueprint/Systems/DayCycle/WB_EndDay Object Reference"))
  (`Widget.SetVisibility` (`/Game/Blueprint/Systems/DayCycle/WB_PlayerUI.ClockText` (`self.ClockWidget`)) "Hidden")
  (bind _returnvalue (`|CreateWidget` "/Game/Blueprint/Systems/DayCycle/WB_EndDay.WB_EndDay_C"))
  (bind _output_get (set `local.DayEndWidget` _returnvalue))
  (`UserWidget.AddToViewport` _output_get 0)
  (`self.WidgetInputSet` _returnvalue)
  (`self.ConstructWidget` _returnvalue)
  (set `self.IsClockActive` false))

(fn `InitializeClockWidget`
  (params (Widget :type "/Game/Blueprint/Systems/DayCycle/WB_PlayerUI Object Reference"))
  (`Widget.SetVisibility` (`/Game/Blueprint/Systems/DayCycle/WB_PlayerUI.ClockText` Widget) "Hidden")
  (`UserWidget.AddToViewport` Widget 0))

(fn `StartDay`
  (bind _gamestate (`self.GameState`))
  (`Widget.SetVisibility` (`/Game/Blueprint/Systems/DayCycle/WB_PlayerUI.ClockText` (`self.ClockWidget`)) "Visible")
  (set `self.CurrentHour` 10)
  (set `self.IsClockActive` true)
  (set `/Game/Blueprint/Systems/BP_Status.DayStartBankPrice` (`/Game/Blueprint/Systems/BP_Status.BankAccount` _gamestate) _gamestate))

(fn `TwoNumber`
  (params (Int :type Integer))
  (returns (Return :type String))
  (bind _returnvalue (`KismetStringLibrary.Conv_IntToString` Int))
  (return (`KismetMathLibrary.SelectString` (`KismetStringLibrary.Concat_StrStr` "0" _returnvalue) _returnvalue (< Int 10))))

(fn `UserConstructionScript`)

(fn `WidgetInputSet`
  (params (Widget :type "UserWidget Object Reference"))
  (`UserWidget.AddToViewport` Widget 0)
  (set `PlayerController.bShowMouseCursor` true (`GameplayStatics.GetPlayerController` 0)))